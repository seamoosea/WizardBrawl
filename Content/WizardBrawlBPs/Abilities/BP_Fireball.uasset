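; BP_Fireball is a fireball ability actor that damages and knocks back what it hits.
; On Hit it ignores its owner apart from a debug print; otherwise it applies damage to the other actor and sends it a HitKBMessage with a brief stun and knockback along the direction from fireball to target.
; It then destroys itself.
; A leftover debug hit chain remains in the graph but never runs.
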(event `self.ReceiveHit`
  (params (MyComp :type "PrimitiveComponent Object Reference") (Other :type "Actor Object Reference") (OtherComp :type "PrimitiveComponent Object Reference") (bSelfMoved :type Boolean) (HitLocation :type "Vector Structure") (HitNormal :type "Vector Structure") (NormalImpulse :type "Vector Structure") (Hit :type "HitResult Structure (by ref)"))
  (if (== Other (`self.GetOwner`))
    (`KismetSystemLibrary.PrintString` "Hit owner")
    (else
      (`GameplayStatics.ApplyDamage` Other 0.0 null self)
      (message `/Game/WizardBrawlBPs/Blueprints/BPI_PlayerCharacter.Hit_KB` Other 0.5 (* (`KismetMathLibrary.GetDirectionUnitVector` (`self.K2_GetActorLocation`) (`self.K2_GetActorLocation` Other)) 1000.0))
      (`self.K2_DestroyActor`))))

(fn `UserConstructionScript`)