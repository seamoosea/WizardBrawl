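; BP_Char is a player-controlled actor that casts a fireball when Q is pressed.
; The Fireball function spawns a BP_Fireball slightly in front of the actor, matching its rotation and adjusting for collisions but always spawning.
; It launches the projectile by adding physics linear velocity to its Capsule along the actor's forward vector, with the vertical component zeroed so the push is horizontal.
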(event `Key|Q`
  (params (Key :type "Key Structure"))
  (:`Pressed`
    (`self.Fireball`)))

(fn `Fireball`
  (bind _returnvalue (`self.K2_GetActorRotation`))
  (bind _returnvalue_2 (`|SpawnActorFromClass` "/Game/WizardBrawlBPs/Abilities/BP_Fireball.BP_Fireball_C" (`KismetMathLibrary.MakeTransform` (+ (`self.K2_GetActorLocation`) (* (`KismetMathLibrary.GetForwardVector` _returnvalue) 50.0)) _returnvalue) "AdjustIfPossibleButAlwaysSpawn" "OverrideRootScale" null null))
  (`PrimitiveComponent.SetAllPhysicsLinearVelocity` (`/Game/WizardBrawlBPs/Abilities/BP_Fireball.Capsule` _returnvalue_2) (* (1000.0 1000.0 0.0) (`KismetMathLibrary.GetForwardVector` (`self.K2_GetActorRotation`))) true))

(fn `UserConstructionScript`)